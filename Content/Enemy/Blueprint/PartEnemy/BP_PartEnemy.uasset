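; BP_PartEnemy is an enemy character that starts in falling movement and damages any actor overlapping its AttackBox.
; Tick aligns the mesh to control rotation with a yaw offset once Target is valid, then disables itself.
; Until then, while Trans is set, it forces the mesh to TargetRot, rotates the capsule and places the mesh at the actor location.
; The RepNotify handlers for Trans and TargetRot are empty.
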(event OnComponentBeginOverlap(AttackBox)
  (params (OverlappedComponent :type Primitive%20Component%20Object%20Reference) (OtherActor :type Actor%20Object%20Reference) (OtherComp :type Primitive%20Component%20Object%20Reference) (OtherBodyIndex :type Integer) (bFromSweep :type Boolean) (SweepResult :type Hit%20Result%20Structure%20%28by%20ref%29))
  (Game|Damage|ApplyDamage OtherActor (Variables|Default|GetAttackDamage) 0 self))

(event EventBeginPlay
  (Pawn|Components|CharacterMovement|SetMovementMode (Variables|Character|GetCharacterMovement) "MOVE_Falling" 0))

(event Collision|EventActorBeginOverlap
  (params (OtherActor :type Actor%20Object%20Reference)))

(event EventTick
  (params (DeltaSeconds :type Float%20%28single-precision%29))
  (Utilities|IsValid (Variables|Default|GetTarget)
    (:Is%20Valid
      (Transformation|SetWorldRotation (Variables|Character|GetMesh) (Math|Rotator|CombineRotators (Pawn|GetControlRotation :!class /Script/Engine.Pawn) "0.000000,-90.000000,0.000000") false false)
      (Actor|Tick|SetActorTickEnabled false))
    (:Is%20Not%20Valid
      (if (Variables|Default|GetTrans)
        (Transformation|SetRelativeTransform (Variables|Character|GetMesh) (Math|Transform|Lerp(Transform) (Math|Transform|MakeTransform (Variables|Default|GettempVec) (Variables|Default|GettempRot) "1.000000,1.000000,1.000000") (Math|Transform|MakeTransform "0, 0, 0" (Variables|Default|GetTargetRot) "1.000000,1.000000,1.000000") 1.0) false false)
        (Transformation|SetWorldRotation (Variables|Default|GetCapsuleComponent) "0.000000,-90.000000,0.000000" false false)
        (Transformation|SetWorldLocation (Variables|Character|GetMesh) (+ (Transformation|GetActorLocation) (Math|Vector|Lerp(Vector) "0, 0, 0" "0.000000,0.000000,-30.000000" 0.0)) false false)))))

(fn ConstructionScript)

(fn OnRepTrans)

(fn OnRepTargetRot)