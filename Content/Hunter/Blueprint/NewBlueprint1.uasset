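; Actor Blueprint in the Hunter folder that handles mouse-wheel quickslot selection.
; Wheel up and down increment or decrement CurQuickKey, with no clamping here, then pass the key's axis value to ChangeQuickslot, whose body is not in this file.
; Both inputs then cast MainUI to WBP_MainUI and refresh its quickslot display.
; BeginPlay, overlap, Tick and the construction script are empty.
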(event EventBeginPlay)

(event Collision|EventActorBeginOverlap
  (params (OtherActor :type Actor%20Object%20Reference)))

(event EventTick
  (params (DeltaSeconds :type Float%20%28single-precision%29)))

(event Input|MouseEvents|MouseWheelUp
  (params (Key :type Key%20Structure :default "None"))
  (:Pressed
    (Variables|Default|SetCurQuickKey (+ (Variables|Default|GetCurQuickKey) 1))
    (Class|Hunter|ChangeQuickslot (Class|Actor|GetInputAxisKeyValue Key))
    (bind _aswbp_main_ui (Utilities|Casting|CastToWBP_MainUI (Variables|Default|GetMainUI)))
    (Default|UpdateQuickSlot _aswbp_main_ui)))

(event Input|MouseEvents|MouseWheelDown
  (params (Key :type Key%20Structure :default "None"))
  (:Pressed
    (Variables|Default|SetCurQuickKey (- (Variables|Default|GetCurQuickKey) 1))
    (Class|Hunter|ChangeQuickslot (Class|Actor|GetInputAxisKeyValue Key))
    (bind _aswbp_main_ui (Utilities|Casting|CastToWBP_MainUI (Variables|Default|GetMainUI)))
    (Default|UpdateQuickSlot _aswbp_main_ui)))

(fn ConstructionScript)