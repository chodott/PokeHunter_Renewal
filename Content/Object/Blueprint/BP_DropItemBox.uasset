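; BP_DropItemBox is a dropped item box that pops upward, tumbles through the air and settles where it lands.
; BeginPlay applies an upward velocity impulse to the physics mesh, and Tick spins it on pitch and yaw.
; A hit while simulating calls ServerOnHit, which relays to MultiOnHit to stop tick and physics, align the mesh to the hit normal, lower it and reposition the actor.
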(event OnComponentHit(StaticMesh)
  (params (HitComponent :type Primitive%20Component%20Object%20Reference) (OtherActor :type Actor%20Object%20Reference) (OtherComp :type Primitive%20Component%20Object%20Reference) (NormalImpulse :type Vector :default "0, 0, 0") (Hit :type Hit%20Result%20Structure%20%28by%20ref%29))
  (if (Physics|IsSimulatingPhysics (Variables|Default|GetStaticMesh) "None")
    (CallFunction|ServeronHit)))

(event Custom|MultiOnHit
  (bind _staticmesh (Variables|Default|GetStaticMesh))
  (bind _returnvalue (Transformation|GetWorldLocation _staticmesh))
  (bind _returnvalue_2 (- _returnvalue "0.000000,0.000000,20.000000"))
  (Actor|Tick|SetActorTickEnabled false)
  (Physics|SetSimulatePhysics (Variables|Default|GetStaticMesh) false)
  (Transformation|SetRelativeRotation (Variables|Default|GetStaticMesh) (Math|Rotator|MakeRotfromZX (.normal (stale OnComponentHit(StaticMesh) Hit)) (Transformation|GetActorForwardVector)) false false)
  (Transformation|SetWorldLocation (Variables|Default|GetStaticMesh) _returnvalue_2 false false)
  (Transformation|SetActorLocation _returnvalue_2 false false))

(event Custom|ServerOnHit
  (CallFunction|MultionHit))

(event EventBeginPlay
  (Physics|AddImpulse (Variables|Default|GetStaticMesh) "0.000000,0.000000,1000.000000" "None" true))

(event Collision|EventActorBeginOverlap
  (params (OtherActor :type Actor%20Object%20Reference)))

(event EventTick
  (params (DeltaSeconds :type Float%20%28single-precision%29))
  (bind _returnvalue (* DeltaSeconds 1e+03))
  (Transformation|AddLocalRotation (Variables|Default|GetStaticMesh) (Math|Rotator|MakeRotator 0.0 _returnvalue _returnvalue) false false))

(fn ConstructionScript)