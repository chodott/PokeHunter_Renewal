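; BP_DefaultEnemy is an enemy character with a sword attack, damage feedback and knockback.
; Its sword hitbox applies AttackDamage to overlapping actors, and damage events spawn a viewport widget showing the amount at the hit location.
; Radial damage launches it away from the blast origin.
; The construction script sizes a sphere to AttackRange and records its starting location as BaseLocation.
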(event OnComponentBeginOverlap(SwordBox)
  (params (OverlappedComponent :type Primitive%20Component%20Object%20Reference) (OtherActor :type Actor%20Object%20Reference) (OtherComp :type Primitive%20Component%20Object%20Reference) (OtherBodyIndex :type Integer) (bFromSweep :type Boolean) (SweepResult :type Hit%20Result%20Structure%20%28by%20ref%29))
  (Game|Damage|ApplyDamage OtherActor (Variables|Default|GetAttackDamage) (Pawn|GetController) 0 "/Script/Engine.DamageType"))

(event Custom|ShowDamage
  (params (DamageAmount :type Float%20%28single-precision%29) (HitLoc :type Vector))
  (bind _returnvalue (UserInterface|CreateWidget "/Game/UI/WBP_DamageDisplay.WBP_DamageDisplay_C" 0 DamageAmount HitLoc))
  (UserInterface|Viewport|AddtoViewport _returnvalue 0))

(event EventBeginPlay
  (EventDispatchers|BindEventtoOnDamage (delegate Custom|ShowDamage)))

(event Collision|EventActorBeginOverlap
  (params (OtherActor :type Actor%20Object%20Reference)))

(event EventTick
  (params (DeltaSeconds :type Float%20%28single-precision%29)))

(event Game|Damage|EventRadialDamage
  (params (DamageReceived :type Float%20%28single-precision%29) (DamageType :type Damage%20Type%20Object%20Reference) (Origin :type Vector :default "0, 0, 0") (HitInfo :type Hit%20Result%20Structure%20%28by%20ref%29) (InstigatedBy :type Controller%20Object%20Reference) (DamageCauser :type Actor%20Object%20Reference))
  (Character|LaunchCharacter (* (Math|Vector|Normalize (- (Transformation|GetActorLocation) Origin)) 1e+03) true true))

(fn ConstructionScript
  (Components|Sphere|SetSphereRadius (Variables|Default|GetSphere) (Variables|Default|GetAttackRange) true)
  (Variables|Default|SetBaseLocation (Transformation|GetActorLocation)))