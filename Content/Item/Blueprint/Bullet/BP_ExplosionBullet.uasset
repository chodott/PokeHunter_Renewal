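; Explosive bullet Blueprint that deals radial damage and plays a world camera shake at its mesh location.
; Its sphere starts with collision disabled; ApplyAbillity enables it, explodes, then launches overlapping Characters along a rotated direction derived from their offset to the bullet.
; OnHitNotEnemy triggers only the damage and shake, without knockback.
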(event EventBeginPlay
  (Collision|SetCollisionEnabled (Variables|Default|GetSphere) "NoCollision"))

(event Collision|EventActorBeginOverlap
  (params (OtherActor :type Actor%20Object%20Reference)))

(event EventTick
  (params (DeltaSeconds :type Float%20%28single-precision%29)))

(event EventApplyAbillity
  (params (OtherActor :type Actor%20Object%20Reference) (OtherComponent :type Primitive%20Component%20Object%20Reference))
  (bind _staticmesh (Variables|Default|GetStaticMesh))
  (bind _returnvalue (Transformation|GetWorldLocation _staticmesh))
  (Collision|SetCollisionEnabled (Variables|Default|GetSphere) "QueryAndPhysics")
  (Game|Damage|ApplyRadialDamage 1e+01 _returnvalue 5e+02 "/Script/Engine.DamageType" 0 0 0 false "ECC_GameTraceChannel8")
  (Camera|PlayWorldCameraShake "/Game/Item/Blueprint/Bullet/BP_ExplosionCameraShake.BP_ExplosionCameraShake_C" _returnvalue 0.0 5e+03)
  (for _array_element (Collision|GetOverlappingActors (Variables|Default|GetSphere) "/Script/Engine.Character" :!class /Script/Engine.PrimitiveComponent)
    (bind _ascharacter (Utilities|Casting|CastToCharacter _array_element))
    (Character|LaunchCharacter _ascharacter (Math|Vector|RotateVector (* (Math|Vector|Normalize (- (Transformation|GetActorLocation _ascharacter) _returnvalue)) 1e+03) "60.000000,0.000000,0.000000") false false)))

(event EventOnHitNotEnemy
  (params (HitVec :type Vector%20%28by%20ref%29 :default "0, 0, 0"))
  (bind _staticmesh (Variables|Default|GetStaticMesh))
  (bind _returnvalue (Transformation|GetWorldLocation _staticmesh))
  (Game|Damage|ApplyRadialDamage 1e+01 _returnvalue 5e+02 "/Script/Engine.DamageType" 0 0 0 false "ECC_GameTraceChannel8")
  (Camera|PlayWorldCameraShake "/Game/Item/Blueprint/Bullet/BP_ExplosionCameraShake.BP_ExplosionCameraShake_C" _returnvalue 0.0 5e+03))

(fn ConstructionScript)