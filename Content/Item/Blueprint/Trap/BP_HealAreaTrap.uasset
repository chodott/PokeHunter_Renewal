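; Heal area trap that affects actors entering and leaving its collision box.
; Begin overlap routes through ApplyAbillity, which sends InteractHealAreaMessage to the entering actor, leaving the response to the receiver.
; End overlap casts to Hunter and subtracts a hardcoded amount from HealPerSecondAmount; the matching increase is not in this Blueprint.
; Tick loops over overlapping Pawns but does nothing with them.
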(event OnComponentBeginOverlap(CollisionBox)
  (params (OverlappedComponent :type Primitive%20Component%20Object%20Reference) (OtherActor :type Actor%20Object%20Reference) (OtherComp :type Primitive%20Component%20Object%20Reference) (OtherBodyIndex :type Integer) (bFromSweep :type Boolean) (SweepResult :type Hit%20Result%20Structure%20%28by%20ref%29))
  (Class|Item|ApplyAbillity OtherActor OtherComp))

(event OnComponentEndOverlap(CollisionBox)
  (params (OverlappedComponent :type Primitive%20Component%20Object%20Reference) (OtherActor :type Actor%20Object%20Reference) (OtherComp :type Primitive%20Component%20Object%20Reference) (OtherBodyIndex :type Integer))
  (bind _ashunter (Utilities|Casting|CastToHunter OtherActor))
  (Variables|/Script/PokeHunter.Hunter|SetHealPerSecondAmount _ashunter (- (Variables|/Script/PokeHunter.Hunter|GetHealPerSecondAmount _ashunter) 1e+01)))

(event EventBeginPlay)

(event Collision|EventActorBeginOverlap
  (params (OtherActor :type Actor%20Object%20Reference)))

(event EventTick
  (params (DeltaSeconds :type Float%20%28single-precision%29))
  (for _array_element (Collision|GetOverlappingActors (Variables|Default|GetCollisionBox) "/Script/Engine.Pawn" :!class /Script/Engine.PrimitiveComponent)
    _))

(event EventApplyAbillity
  (params (OtherActor :type Actor%20Object%20Reference) (OtherComponent :type Primitive%20Component%20Object%20Reference))
  (Class|ItemInteractInterface|InteractHealArea(Message) OtherActor))

(fn ConstructionScript)